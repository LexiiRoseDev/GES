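; BP_AIMelee is a melee AI Blueprint that deals repeated damage to the player on contact.
; Overlapping DmgCol with a "Player"-tagged actor applies DmgVal immediately, then loops through a one-second Delay while IsOverlap stays true.
; End overlap clears that flag to end the loop.
; BeginPlay caches the player character, though the damage logic relies only on the tag, and its game mode cast result is unused.
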(event OnComponentBeginOverlap(DmgCol)
  (params (OverlappedComponent :type Primitive%20Component%20Object%20Reference) (OtherActor :type Actor%20Object%20Reference) (OtherComp :type Primitive%20Component%20Object%20Reference) (OtherBodyIndex :type Integer) (bFromSweep :type Boolean) (SweepResult :type Hit%20Result%20Structure%20%28by%20ref%29))
  ;[0.15 0.15 0.15 0.5] Detects whether overlapping component is the player and checks if player is dead or alive.
  (if (Actor|ActorHasTag OtherActor "Player")
    (Variables|Default|SetisOverlap true)
    (Game|Damage|ApplyDamage OtherActor (Variables|Default|GetDmgVal) 0 0 :!label _label)
    (if (Variables|Default|GetisOverlap)
      (Utilities|FlowControl|Delay 1.0)
      (goto _label))))

(event OnComponentEndOverlap(DmgCol)
  (params (OverlappedComponent :type Primitive%20Component%20Object%20Reference) (OtherActor :type Actor%20Object%20Reference) (OtherComp :type Primitive%20Component%20Object%20Reference) (OtherBodyIndex :type Integer))
  (if (Actor|ActorHasTag OtherActor "Player")
    (Variables|Default|SetisOverlap false)))

(event EventBeginPlay
  ;[0.15 0.15 0.15 0.5] Set player reference upon begin play.
  (Utilities|FlowControl|Sequence
    (:then_0
      (bind _asbp_third_person_character (Utilities|Casting|CastToBP_ThirdPersonCharacter (Game|GetPlayerCharacter 0)))
      (Utilities|IsValid _asbp_third_person_character
        (:Is%20Valid
          (Variables|Default|SetPlayer _asbp_third_person_character)
          (Development|PrintString "Player set!"))
        (:Is%20Not%20Valid
          (Development|PrintString "No Player found"))))
    (:then_1
      (Utilities|Casting|CastToBP_ThirdPersonGameMode (Game|GetGameMode)))))

(event EventTick
  (params (DeltaSeconds :type Float%20%28single-precision%29)))

(fn ConstructionScript)