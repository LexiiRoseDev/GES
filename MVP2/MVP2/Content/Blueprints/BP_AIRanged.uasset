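; BP_AIRanged is a ranged AI enemy that idly rotates until its perception updates, then faces the player.
; On any perception update it prints a debug message, turns toward player 0's ThirdPersonCharacter and deactivates its RotatingMovement.
; It then starts a looping timer with no visible bound event and spawns one actor at its location, aimed at the player.
; The spawned class is unspecified, and the sensed actor and stimulus are ignored.
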(event OnTargetPerceptionUpdated(AIPerception)
  (params (Actor :type Actor%20Object%20Reference) (Stimulus :type AI%20Stimulus%20Structure))
  (bind _self self)
  (bind _returnvalue (Transformation|GetActorTransform _self))
  (Development|PrintString "I see you!")
  (bind _asbp_third_person_character (Utilities|Casting|CastToBP_ThirdPersonCharacter (Game|GetPlayerCharacter 0)))
  (Transformation|SetActorRotation (Math|Rotator|FindLookatRotation (Transformation|GetActorLocation _self) (Transformation|GetActorLocation _asbp_third_person_character)))
  (Components|Activation|Deactivate (Variables|Default|GetRotatingMovement))
  (Utilities|Time|SetTimerbyEvent 0 1.0 true)
  (Game|SpawnActorfromClass "/Game/Blueprints/BP_Projectile.BP_Projectile_C" (Math|Transform|MakeTransform (.location _returnvalue) (Math|Rotator|FindLookatRotation (Transformation|GetActorLocation _self) (Transformation|GetActorLocation _asbp_third_person_character)) (.scale _returnvalue)) "Undefined" "MultiplyWithRoot" 0 0))

(event EventTick
  (params (DeltaSeconds :type Float%20%28single-precision%29)))

(fn ConstructionScript)