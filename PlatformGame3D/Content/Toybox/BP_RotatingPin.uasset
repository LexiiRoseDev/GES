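; BP_RotatingPin is a Toybox object that spins items around a central pole and can be started or stopped by a linked button.
; While IsRotating is set, Tick yaws CentralPost locally by RotationSpeed scaled by delta time.
; The Switchon and SwitchOff events set IsRotating, with DoesSwitchDeactivate inverting them so the switch can stop the rotation instead of starting it.
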(event EventBeginPlay)

(event Collision|EventActorBeginOverlap
  (params (OtherActor :type Actor%20Object%20Reference)))

(event EventTick
  (params (DeltaSeconds :type Float%20%28single-precision%29))
  ;[1 1 1] If turned on rotate the objects around the pole
  (if (Variables|Default|GetIsRotating)
    (Transformation|AddLocalRotation (Variables|Default|GetCentralPost) (Math|Rotator|MakeRotator 0.0 0.0 (* DeltaSeconds (Variables|Default|GetRotationSpeed))) false false)))

(event EventSwitchon
  ;[1 1 1] If linked to a buton, start / stop rotating based on the button press
  (if (Variables|Default|GetDoesSwitchDeactivate)
    (Variables|Default|SetIsRotating false)
    (else
      (Variables|Default|SetIsRotating true))))

(event EventSwitchOff
  ;[1 1 1] If linked to a buton, start / stop rotating based on the button press
  (if (Variables|Default|GetDoesSwitchDeactivate)
    (Variables|Default|SetIsRotating true)
    (else
      (Variables|Default|SetIsRotating false))))

(fn ConstructionScript)