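; BP_Button is a pressure button that switches a list of controlled actors on and off through BPI_ButtonInterface.
; BeginPlay calculates the pressed position and switches targets off, printing an error and destroying the button if any target is invalid or lacks the interface.
; Trigger overlap counts filter out extra overlaps, swapping the material, messaging targets and driving a Timeline that moves the top.
; Release only switches off when CanTurnOff is set.
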(event OnComponentBeginOverlap(SwitchTrigger)
  (params (OverlappedComponent :type Primitive%20Component%20Object%20Reference) (OtherActor :type Actor%20Object%20Reference) (OtherComp :type Primitive%20Component%20Object%20Reference) (OtherBodyIndex :type Integer) (bFromSweep :type Boolean) (SweepResult :type Hit%20Result%20Structure%20%28by%20ref%29))
  ;[1 1 1] Check to see if we are the only object being considered (if something else is allready overlapping, we should ignore this!
  (if (== (Utilities|Array|Length (Collision|GetOverlappingActors (Variables|Default|GetSwitchTrigger) 0 :!class /Script/Engine.PrimitiveComponent)) 2)
    ;[1 1 1] Set the button colour
    (Rendering|Material|SetMaterial (Variables|Default|GetSM_ButtonTop) 0 (Variables|Default|GetOn%20Colour))
    ;[1 1 1] For each actor connected to the button...
    (for _array_element (Variables|Default|GetControlled%20Actors)
      ;[1 1 1] Check to see if the object is still attached to the switch
      (Utilities|IsValid _array_element
        (:Is%20Valid
          ;[1 1 1] Switch the targeted object on or off
          (Class|BPIButtonInterface|Switchon(Message) _array_element))))
    ;[1 1 1] Animate Button for on and off
    (bind _movement (Timeline|Timeline Play)
      (:Update
        (Transformation|SetWorldTransform (Variables|Default|GetSM_ButtonTop) (Math|Transform|Lerp(Transform) (Variables|Default|GetOff%20Position) (Variables|Default|GetOn%20Position) _movement) false false)))))

(event OnComponentEndOverlap(SwitchTrigger)
  (params (OverlappedComponent :type Primitive%20Component%20Object%20Reference) (OtherActor :type Actor%20Object%20Reference) (OtherComp :type Primitive%20Component%20Object%20Reference) (OtherBodyIndex :type Integer))
  (if (Variables|Default|GetCan%20Turn%20Off)
    ;[1 1 1] Check to see if we are the only object being considered (if something else is allready overlapping, we should ignore this!
    (if (== (Utilities|Array|Length (Collision|GetOverlappingActors (Variables|Default|GetSwitchTrigger) 0 :!class /Script/Engine.PrimitiveComponent)) 1)
      ;[1 1 1] Set the button colour
      (Rendering|Material|SetMaterial (Variables|Default|GetSM_ButtonTop) 0 (Variables|Default|GetOff%20Colour))
      ;[1 1 1] For each actor connected to the button...
      (for _array_element (Variables|Default|GetControlled%20Actors)
        ;[1 1 1] Check to see if the object is still attached to the switch
        (Utilities|IsValid _array_element
          (:Is%20Valid
            ;[1 1 1] Switch the targeted object on or off
            (Class|BPIButtonInterface|SwitchOff(Message) _array_element))))
      ;[1 1 1] Animate Button for on and off
      (bind _movement (Timeline|Timeline Reverse)
        (:Update
          (Transformation|SetWorldTransform (Variables|Default|GetSM_ButtonTop) (Math|Transform|Lerp(Transform) (Variables|Default|GetOff%20Position) (Variables|Default|GetOn%20Position) _movement) false false))))))

(event EventBeginPlay
  ;[1 1 1] Set the off position of the button
  (Variables|Default|SetOff%20Position (Transformation|GetWorldTransform (Variables|Default|GetSM_ButtonTop)))
  ;[1 1 1] Calculate the button on position and set it
  (Variables|Default|SetOn%20Position (Math|Transform|MakeTransform (+ (* (Math|Vector|GetUpVector (Variables|Default|GetSM_ButtonTop)) -9.0) (.location (Variables|Default|GetOff%20Position))) (.rotation (Variables|Default|GetOff%20Position)) (.scale (Variables|Default|GetOff%20Position))))
  ;[1 1 1] Check all actors attached to the button exist and can be switched on and off
  (for _array_element (Variables|Default|GetControlled%20Actors)
    (Utilities|IsValid _array_element
      (:Is%20Valid
        (if (Utilities|DoesObjectImplementInterface _array_element "/Game/Interfaces/BPI_ButtonInterface.BPI_ButtonInterface_C")
          (Class|BPIButtonInterface|SwitchOff(Message) _array_element) ; Switch off the object attached to the button
          (else
            (CallFunction|DebugMissingInterface))))
      (:Is%20Not%20Valid
        (CallFunction|DebugMissingObject))))
  ;[1 1 1] Set the button colour
  (Rendering|Material|SetMaterial (Variables|Default|GetSM_ButtonTop) 0 (Variables|Default|GetOff%20Colour)))

(event Collision|EventActorBeginOverlap
  (params (OtherActor :type Actor%20Object%20Reference)))

(event EventTick
  (params (DeltaSeconds :type Float%20%28single-precision%29)))

(fn ConstructionScript)

(fn DebugMissingObject
  (bind _self self)
  (bind _returnvalue (Utilities|GetDisplayName _self))
  (Development|PrintString (Utilities|String|Append _returnvalue " has no object to control, please provide an actor for me to control! || " _returnvalue " has been destroyed to prevent errors") true false "(R=1.000000,G=0.000000,B=0.015913,A=1.000000)" 1e+03)
  (Actor|DestroyActor))

(fn DebugMissingInterface
  (bind _self self)
  (bind _returnvalue (Utilities|GetDisplayName _self))
  (Development|PrintString (Utilities|String|Append "The object selected as a target for " _returnvalue " does not implement the button interface :( || please let the person running the session when you have a moment :) || " _returnvalue " has been destroyed to prevent errors") true false "(R=1.000000,G=0.000000,B=0.015913,A=1.000000)" 1e+03)
  (Actor|DestroyActor))