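; BP_Crystal is a collectible crystal that adds PointsValue to the score of an overlapping BP_ThirdPersonCharacter, then destroys itself.
; The SpinAndBob timeline yaws the mesh and applies a sine bob around its captured start point, with a random start time to desynchronise crystals.
; Switchon and SwitchOff events set IsHidden, which HideRevealCrystal applies to visibility and collision, also on BeginPlay.
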(event OnComponentBeginOverlap(StaticMeshComponent)
  (params (OverlappedComponent :type Primitive%20Component%20Object%20Reference) (OtherActor :type Actor%20Object%20Reference) (OtherComp :type Primitive%20Component%20Object%20Reference) (OtherBodyIndex :type Integer) (bFromSweep :type Boolean) (SweepResult :type Hit%20Result%20Structure%20%28by%20ref%29))
  ;[1 1 1] If i touch the player, score 5 points
  (bind _asbp_third_person_character (Utilities|Casting|CastToBP_ThirdPersonCharacter OtherActor))
  (Default|AddScore _asbp_third_person_character (Variables|Properties|GetPointsValue))
  (Actor|DestroyActor) ; then destory myself
)

(event EventBeginPlay
  (bind _spin_and_bob (Variables|Default|GetSpin%20and%20bob))
  ;[0.15 0.15 0.15 0.5] Capture the starting point for the crystal so we have a central point to "bob" around.
  (Variables|Default|SetObjectStartPoint (Transformation|GetActorLocation))
  ;[0.15 0.15 0.15 0.5] Set the visability and rotation speed of the crystal and set a random starting offset (so all crystals start at different rotations)
  (CallFunction|Hide/RevealCrystal)
  (Components|Timeline|SetPlayRate _spin_and_bob (Variables|CrystalSettings|GetRotationSpeed))
  (Components|Timeline|SetNewTime _spin_and_bob (Math|Random|RandomFloat))
  (Utilities|FlowControl|DelayUntilNextTick)
  (bind _value (Timeline|Spin%20and%20bob Play) ; Timeline counts from 0 to 1 each duration.
    (:Update
      (Transformation|SetRelativeLocationAndRotation (Variables|Debug|GetStaticMeshComponent) (Math|Vector|MakeVector (.x (Variables|Default|GetObjectStartPoint)) (.y (Variables|Default|GetObjectStartPoint)) (+ (.z (Variables|Default|GetObjectStartPoint)) (* (- (Math|Trig|Sin(Degrees) (* _value 3.6e+02)) 0.5) (Variables|CrystalSettings|GetBob%20Amount)))) (Math|Rotator|MakeRotator 0.0 0.0 (* _value 3.6e+02)) false false) ; Apply crystal movement
    )))

(event EventSwitchon
  (Variables|Default|SetIsHidden false)
  (CallFunction|Hide/RevealCrystal))

(event EventSwitchOff
  (Variables|Default|SetIsHidden true)
  (CallFunction|Hide/RevealCrystal))

(fn ConstructionScript)

(fn Hide/RevealCrystal
  (bind _ishidden (Variables|Default|GetIsHidden))
  (Rendering|SetActorHiddenInGame self _ishidden)
  (Collision|SetActorEnableCollision (not _ishidden)))