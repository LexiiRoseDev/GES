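; BP_Checkpoint is a checkpoint actor that sets the player's spawn point and has a flag that can be raised or lowered.
; When BP_ThirdPersonCharacter overlaps its Trigger, it passes itself to the character's SetNewSpawn.
; RaiseFlag plays a Timeline that lerps the Flag's relative transform from FlagLowered to FlagRaised, and LowerFlag reverses it.
; The overlap does not call either flag event directly.
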(event OnComponentBeginOverlap(Trigger)
  (params (OverlappedComponent :type Primitive%20Component%20Object%20Reference) (OtherActor :type Actor%20Object%20Reference) (OtherComp :type Primitive%20Component%20Object%20Reference) (OtherBodyIndex :type Integer) (bFromSweep :type Boolean) (SweepResult :type Hit%20Result%20Structure%20%28by%20ref%29))
  (bind _asbp_third_person_character (Utilities|Casting|CastToBP_ThirdPersonCharacter OtherActor)) ; check if its the player
  (Default|SetNewSpawn _asbp_third_person_character self) ; if it is, set the spawn to here!
)

(event Custom|Raise%20Flag
  ;[1 1 1] Animate the flag using a timeline
  (bind _time (Timeline|Timeline Play)
    (:Update
      (Transformation|SetRelativeTransform (Variables|Default|GetFlag) (Math|Transform|Lerp(Transform) (Variables|Default|GetFlagLowered) (Variables|Default|GetFlagRaised) _time) false false))))

(event Custom|Lower%20Flag
  ;[1 1 1] Animate the flag using a timeline
  (bind _time (Timeline|Timeline Reverse)
    (:Update
      (Transformation|SetRelativeTransform (Variables|Default|GetFlag) (Math|Transform|Lerp(Transform) (Variables|Default|GetFlagLowered) (Variables|Default|GetFlagRaised) _time) false false))))

(event EventBeginPlay)

(event Collision|EventActorBeginOverlap
  (params (OtherActor :type Actor%20Object%20Reference)))

(event EventTick
  (params (DeltaSeconds :type Float%20%28single-precision%29)))

(fn ConstructionScript)