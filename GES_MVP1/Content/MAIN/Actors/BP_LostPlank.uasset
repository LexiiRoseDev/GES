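; BP_LostPlank is an actor that provides a replacement plank when the player's plank is flagged as lost.
; While LostPlank is true, Tick reveals the Widget component, using IsVis to do so only once.
; Each player overlap with BoxColl then spawns a BP_Plank at a hardcoded world location.
; Nothing here sets or clears LostPlank, so repeated overlaps can spawn more planks while it stays true.
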(event OnComponentBeginOverlap(BoxColl)
  (params (OverlappedComponent :type Primitive%20Component%20Object%20Reference) (OtherActor :type Actor%20Object%20Reference) (OtherComp :type Primitive%20Component%20Object%20Reference) (OtherBodyIndex :type Integer) (bFromSweep :type Boolean) (SweepResult :type Hit%20Result%20Structure%20%28by%20ref%29))
  (Utilities|Casting|CastToBP_ThirdPersonCharacter OtherActor)
  (if (Variables|Default|GetlostPlank)
    (Game|SpawnActorfromClass "/Game/MAIN/Actors/BP_Plank.BP_Plank_C" (Math|Conversions|ToTransform(Vector) "0.000000,-1640.000000,0.000000") "Undefined" "MultiplyWithRoot" 0 0)))

(event EventBeginPlay)

(event Collision|EventActorBeginOverlap
  (params (OtherActor :type Actor%20Object%20Reference)))

(event EventTick
  (params (DeltaSeconds :type Float%20%28single-precision%29))
  (if (Variables|Default|GetlostPlank)
    (if (not (Variables|Default|GetisVis))
      (Rendering|SetVisibility (Variables|Default|GetWidget) true false)
      (Variables|Default|SetisVis true))))

(fn ConstructionScript)